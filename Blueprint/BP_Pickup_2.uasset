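; BP_Pickup_2 is a collectible that adds a random amount of score, shown to the player as "Laughter".
; A timeline started on BeginPlay moves the Sphere component vertically.
; When the third-person character overlaps Sphere1, it increases Score on the BP_GameStart actor found by class lookup, prints the new total and destroys itself.
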(event OnComponentBeginOverlap(Sphere1)
  (params (OverlappedComponent :type Primitive%20Component%20Object%20Reference) (OtherActor :type Actor%20Object%20Reference) (OtherComp :type Primitive%20Component%20Object%20Reference) (OtherBodyIndex :type Integer) (bFromSweep :type Boolean) (SweepResult :type Hit%20Result%20Structure%20%28by%20ref%29))
  (Utilities|Casting|CastToBP_ThirdPersonCharacter OtherActor)
  (bind _returnvalue (Actor|GetActorOfClass "/Game/Blueprint/BP_GameStart.BP_GameStart_C"))
  (bind _output_get (Variables|/Game/Blueprint/BP_GameStart.BP_GameStart_C|SetScore _returnvalue (+ (Variables|/Game/Blueprint/BP_GameStart.BP_GameStart_C|GetScore _returnvalue) (Math|Random|RandomIntegerinRange 50 75))))
  (Development|PrintString (Utilities|String|Append "You have collected: " (Utilities|String|ToString(Integer) _output_get) " Laughter!"))
  (Actor|DestroyActor))

(event EventBeginPlay
  (bind _movement (Timeline|PointMovement Play)
    (:Update
      (Transformation|SetRelativeLocation (Variables|Default|GetSphere) (Math|Vector|MakeVector 0.0 0.0 (+ (* _movement 1e+02) 5e+01)) false false))))

(event Collision|EventActorBeginOverlap
  (params (OtherActor :type Actor%20Object%20Reference)))

(event EventTick
  (params (DeltaSeconds :type Float%20%28single-precision%29)))

(fn ConstructionScript)